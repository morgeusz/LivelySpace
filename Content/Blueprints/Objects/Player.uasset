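; Penguin player that hops one grid cell at a time with WASD while grounded.
; GetEndPoint offsets the mesh position by one fixed step, and MovePlayer plays the MoveXYZ timeline to lerp there with a height arc and squeeze scaling, blocking input until it lands.
; While grounded, FixPosition runs on Tick to rest the mesh on the pad at its grid coordinates, looked up in GameModeInGame's pad lists.
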(event `Key|W`
  (params (Key :type "Key Structure"))
  (:`Pressed`
    (if (`self.isGrounded`)
      (bind (_startcoords _endcoords) (`self.GetEndPoint` 1))
      (`self.MovePlayer` _startcoords _endcoords))))

(event `Key|A`
  (params (Key :type "Key Structure"))
  (:`Pressed`
    (if (`self.isGrounded`)
      (bind (_startcoords _endcoords) (`self.GetEndPoint` 2))
      (`self.MovePlayer` _startcoords _endcoords))))

(event `Key|S`
  (params (Key :type "Key Structure"))
  (:`Pressed`
    (if (`self.isGrounded`)
      (bind (_startcoords _endcoords) (`self.GetEndPoint` 3))
      (`self.MovePlayer` _startcoords _endcoords))))

(event `Key|D`
  (params (Key :type "Key Structure"))
  (:`Pressed`
    (if (`self.isGrounded`)
      (bind (_startcoords _endcoords) (`self.GetEndPoint` 4))
      (`self.MovePlayer` _startcoords _endcoords))))

(event `self.ReceiveTick`
  (params (DeltaSeconds :type "Float (single-precision)"))
  (`self.FixPosition`))

(event `MovePlayer`
  (params (startCoords :type "Vector Structure") (endCoords :type "Vector Structure"))
  (bind _staticmesh (`self.StaticMesh`))
  (set `self.isGrounded` false)
  (bind (_direction _alpha _height _squeeze) (`Timeline|MoveX/Y/Z` :!via `PlayFromStart`)
    (:`Update`
      (bind (_returnvalue_x _returnvalue_y) (`KismetMathLibrary.BreakVector` (`KismetMathLibrary.VLerp` startCoords endCoords _alpha)))
      (`SceneComponent.K2_SetWorldLocation` _staticmesh (`KismetMathLibrary.MakeVector` _returnvalue_x _returnvalue_y (+ _height (.z startCoords))) false false)
      (`SceneComponent.SetWorldScale3D` (`self.StaticMesh`) (* (`self.playerStartScale`) _squeeze)))
    (:`Finished`
      (`SceneComponent.K2_SetWorldLocation` _staticmesh endCoords false false)
      (set `self.isGrounded` true))))

(fn `FixPosition`
  (bind _staticmesh (`self.StaticMesh`))
  (bind _gamemoderef (`self.gameModeREF`))
  (bind (_returnvalue_x _returnvalue_y) (`KismetMathLibrary.BreakVector` (`SceneComponent.K2_GetComponentLocation` _staticmesh)))
  (bind (_returnvalue_x_2 _returnvalue_y_2 _returnvalue_z) (`KismetMathLibrary.BreakVector` (`SceneComponent.K2_GetComponentLocation` (`/Game/Blueprints/Objects/ObjectPad.Scene` (`|GetArrayItem` (`/Game/Blueprints/Gamemodes/GameModeInGame.padListReferences` _gamemoderef) (`KismetArrayLibrary.Array_Find` (`/Game/Blueprints/Gamemodes/GameModeInGame.padListCoords` _gamemoderef) (`KismetMathLibrary.MakeVector2D` (/ _returnvalue_x 19.0) (/ _returnvalue_y 19.0))))))))
  (if (`self.isGrounded`)
    (`SceneComponent.K2_SetWorldLocation` _staticmesh (`KismetMathLibrary.MakeVector` _returnvalue_x _returnvalue_y (+ _returnvalue_z (.z (`.BoxExtent` (`KismetSystemLibrary.GetComponentBounds` (`self.StaticMesh`)))))) false false)))

(fn `GetEndPoint`
  (params (direction :type Integer))
  (returns (startCoords :type "Vector Structure") (endCoords :type "Vector Structure"))
  (locals (startPoint :type "Vector Structure") (endPoint :type "Vector Structure"))
  (bind _staticmesh (`self.StaticMesh`))
  (bind (_returnvalue_x _returnvalue_y _returnvalue_z) (`KismetMathLibrary.BreakVector` (`SceneComponent.K2_GetComponentLocation` _staticmesh)))
  (set `local.startPoint` (`SceneComponent.K2_GetComponentLocation` _staticmesh))
  (if (== direction 1)
    (set `local.endPoint` (`KismetMathLibrary.MakeVector` (+ _returnvalue_x 19.0) _returnvalue_y _returnvalue_z))
    (return (`local.startPoint`) (`local.endPoint`))
    (elif (== direction 2)
      (set `local.endPoint` (`KismetMathLibrary.MakeVector` _returnvalue_x (- _returnvalue_y 19.0) _returnvalue_z))
      (return (`local.startPoint`) (`local.endPoint`))
      (elif (== direction 3)
        (set `local.endPoint` (`KismetMathLibrary.MakeVector` (- _returnvalue_x 19.0) _returnvalue_y _returnvalue_z))
        (return (`local.startPoint`) (`local.endPoint`))
        (elif (== direction 4)
          (set `local.endPoint` (`KismetMathLibrary.MakeVector` _returnvalue_x (+ _returnvalue_y 19.0) _returnvalue_z))
          (return (`local.startPoint`) (`local.endPoint`)))))))

(fn `UserConstructionScript`
  (bind _staticmesh (`self.StaticMesh`))
  (bind _asgame_mode_in_game (cast `/Game/Blueprints/Gamemodes/GameModeInGame` (`GameplayStatics.GetGameMode`)))
  (set `self.gameModeREF` _asgame_mode_in_game)
  (`StaticMeshComponent.SetStaticMesh` _staticmesh "/Game/Models/Characters/Penguin/pingwin.pingwin")
  (`SceneComponent.K2_SetWorldTransform` _staticmesh (`KismetMathLibrary.MakeTransform` (38.0 38.0 0.0) (struct :`Yaw` 90.0 :`Roll` 90.0)) false false)
  (set `self.playerStartScale` (`SceneComponent.K2_GetComponentScale` (`self.StaticMesh`))))