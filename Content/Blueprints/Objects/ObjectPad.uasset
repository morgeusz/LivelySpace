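; A floating landing pad that reacts when the player lands and temporarily disappears when activated.
; Timelines drive its motion: a looping Z bob with random amplitude and start delay, interrupted by a landing animation that resumes the bob when finished.
; ActivePad plays an XY offset animation around the start position, then hides the pad, clears IsSafe, and restores it after a short delay.
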(event `self.ReceiveBeginPlay`
  (`KismetSystemLibrary.Delay` (`KismetMathLibrary.RandomFloatInRange` 0.0 1.0))
  (`self.float`)
  (`KismetSystemLibrary.Delay` 2.0))

(event `playerLandEffect`
  (bind _scene (`self.Scene`))
  (bind _scene_2 (`self.Scene`))
  (bind (_returnvalue_x _returnvalue_y) (`KismetMathLibrary.BreakVector` (`SceneComponent.K2_GetComponentLocation` _scene)))
  (bind (_returnvalue_x_2 _returnvalue_y_2) (`KismetMathLibrary.BreakVector` (`SceneComponent.K2_GetComponentLocation` _scene_2)))
  (`|ExecutionSequence`
    (:`then_0`
      (bind (_direction _height) (`Timeline|floatEffect` :!via `Stop` :!label _label)
        (:`Update`
          (`SceneComponent.K2_SetWorldLocation` _scene (`KismetMathLibrary.MakeVector` _returnvalue_x _returnvalue_y (* _height (`self.randomFloat`))) false false))
        (:`Finished`
          (`KismetSystemLibrary.Delay` 0.0)
          (goto _label :!via `PlayFromStart`))))
    (:`then_1`
      (bind (_direction_2 _height_2) (`Timeline|landEffect` :!via `PlayFromStart`)
        (:`Update`
          (`SceneComponent.K2_SetWorldLocation` _scene_2 (`KismetMathLibrary.MakeVector` _returnvalue_x_2 _returnvalue_y_2 _height_2) false false))
        (:`Finished`
          (`self.float`))))))

(event `float`
  (goto _label :!via `PlayFromStart`))

(event `ActivePad`
  (bind _scene (`self.Scene`))
  (bind _scene_2 (`self.Scene`))
  (bind (_startposition_x _startposition_y) (`KismetMathLibrary.BreakVector` (`self.startPosition`)))
  (bind (_returnvalue_x _returnvalue_y _returnvalue_z) (`KismetMathLibrary.BreakVector` (`SceneComponent.K2_GetComponentLocation` _scene_2)))
  (`|ExecutionSequence`
    (:`then_0`
      (goto _label :!via `Stop`))
    (:`then_1`
      (bind (_direction _alpha _position) (`Timeline|destroyEffect` :!via `PlayFromStart`)
        (:`Update`
          (`SceneComponent.K2_SetWorldLocation` _scene_2 (`KismetMathLibrary.MakeVector` (+ _startposition_x (./y_x _position)) (+ _startposition_y (./y_y _position)) _returnvalue_z) false false))
        (:`Finished`
          (`SceneComponent.SetVisibility` _scene false true)
          (`SceneComponent.K2_SetWorldLocation` _scene (`self.startPosition`) false false)
          (set `self.isSafe` false)
          (`KismetSystemLibrary.Delay` 1.0)
          (`SceneComponent.SetVisibility` (`self.Scene`) true true)
          (`SceneComponent.K2_SetWorldLocation` (`self.Scene`) (`self.startPosition`) false false)
          (set `self.isSafe` true)
          (goto _label :!via `PlayFromStart`))))))

(fn `UserConstructionScript`
  (bind _returnvalue (`KismetMathLibrary.RandomFloatInRange` 1000.0 10000.0))
  (bind _staticmesh (`self.StaticMesh`))
  (bind (_returnvalue_x _returnvalue_y) (`KismetMathLibrary.BreakVector` (`SceneComponent.K2_GetComponentLocation` _staticmesh)))
  (`StaticMeshComponent.SetStaticMesh` _staticmesh "/Game/Models/Pads/Rocket/RocketPad.RocketPad")
  (`SceneComponent.SetWorldScale3D` (`self.Scene`) (2.0 2.0 2.0))
  (set `self.randomFloat` (`KismetMathLibrary.RandomFloatInRangeFromStream` 0.5 0.75 (`KismetMathLibrary.MakeRandomStream` (`KismetMathLibrary.FTrunc` (+ (* _returnvalue_x _returnvalue) (* _returnvalue_y _returnvalue))))))
  (set `self.startPosition` (`SceneComponent.K2_GetComponentLocation` (`self.Scene`))))