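; In-game GameMode that builds a square grid of ObjectPads, hides the player's scene at start and runs timed pad waves.
; WaveTimer loops WaveMachine at intervals that shrink as TimePlayed rises, choosing random cells, more over time.
; Parallel coordinate and reference arrays map cells to pads for ActivePad, which only runs up to the late-game threshold.
; SpawnObjects is a looping stub for weighted score and money pickups that only prints.
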(event `self.ReceiveBeginPlay`
  (`self.SpawnNet` (`self.netSize`))
  (bind _asplayer (cast `/Game/Blueprints/Objects/Player` (`GameplayStatics.GetPlayerPawn` 0)))
  (bind _output_get (set `self.playerREF` _asplayer))
  (`SceneComponent.SetVisibility` (`/Game/Blueprints/Objects/Player.Scene` _output_get) false true))

(event `self.ReceiveTick`
  (params (DeltaSeconds :type "Float (single-precision)"))
  (if (`self.isGameStarted`)
    (`KismetSystemLibrary.Delay` 1.0)
    (`/Engine/EditorBlueprintResources/StandardMacros.IncrementInt` (`self.timePlayed`))))

(event `WaveTimer`
  (bind _timeplayed (`self.timePlayed`))
  (if (> _timeplayed 100)
    (if (> _timeplayed 300)
      (`KismetSystemLibrary.Delay` 1.0)
      (else
        (`KismetSystemLibrary.Delay` (- 2.0 (/ (- (`KismetMathLibrary.Conv_IntToDouble` (`self.timePlayed`)) 100.0) 200.0)))))
    (else
      (`KismetSystemLibrary.Delay` (- 4.0 (/ (`KismetMathLibrary.Conv_IntToDouble` (`self.timePlayed`)) 50.0)))))
  (`self.WaveMachine`)
  (`self.WaveTimer`))

(event `SpawnObjects`
  (bind _returnvalue (`KismetMathLibrary.RandomIntegerInRange` 1 100))
  (`KismetSystemLibrary.Delay` (`KismetMathLibrary.RandomFloatInRange` 3.0 5.0))
  (if (> _returnvalue 95)
    (`KismetSystemLibrary.PrintString` "Spawned object" :!label _label)
    (`self.SpawnObjects`)
    (elif (> _returnvalue 85)
      (goto _label)
      (elif (> _returnvalue 70)
        (goto _label)
        (elif (> _returnvalue 40)
          (goto _label)
          (elif (> _returnvalue 0)
            (goto _label)))))))

(fn `SpawnNet`
  (params (NetSize :type Integer))
  (bind _returnvalue (- NetSize 1))
  (for _index (range (+ _returnvalue 1))
    (for _index_2 (range (+ _returnvalue 1))
      (`KismetArrayLibrary.Array_Add` (`self.padListCoords`) (`KismetMathLibrary.MakeVector2D` (`KismetMathLibrary.Conv_IntToDouble` _index_2) (`KismetMathLibrary.Conv_IntToDouble` _index)))
      (bind _returnvalue_2 (`|SpawnActorFromClass` "/Game/Blueprints/Objects/ObjectPad.ObjectPad_C" (`KismetMathLibrary.MakeTransform` (`KismetMathLibrary.Conv_IntVectorToVector` (make `IntVector` (* _index_2 19) (* _index 19)))) "AlwaysSpawn" "OverrideRootScale" null null))
      (`KismetArrayLibrary.Array_Add` (`self.padListReferences`) _returnvalue_2)))
  (`KismetSystemLibrary.PrintString` "Koniec renderowania siatki" true true (struct :`R` 1.0 :`A` 1.0) 1.0))

(fn `UserConstructionScript`)

(fn `WaveMachine`
  (bind _padchoosed (`self.padChoosed`))
  (bind _padchoosed_2 (`self.padChoosed`))
  (bind _returnvalue (- (`self.netSize`) 1))
  (bind _returnvalue_2 (- (`self.netSize`) 1))
  (bind _returnvalue_3 (`KismetMathLibrary.MakeVector2D` (`KismetMathLibrary.Conv_IntToDouble` (`KismetMathLibrary.RandomIntegerInRange` 0 _returnvalue)) (`KismetMathLibrary.Conv_IntToDouble` (`KismetMathLibrary.RandomIntegerInRange` 0 _returnvalue))))
  (bind _returnvalue_4 (`KismetMathLibrary.MakeVector2D` (`KismetMathLibrary.Conv_IntToDouble` (`KismetMathLibrary.RandomIntegerInRange` 0 _returnvalue_2)) (`KismetMathLibrary.Conv_IntToDouble` (`KismetMathLibrary.RandomIntegerInRange` 0 _returnvalue_2))))
  (`KismetArrayLibrary.Array_Clear` (`self.padChoosed`))
  (if (> (`self.timePlayed`) 300)
    (for _index (range 1 21)
      (if (== _index 1)
        (`KismetArrayLibrary.Array_Add` _padchoosed_2 _returnvalue_4)
        (else
          (while (== (`KismetArrayLibrary.Array_Find` _padchoosed_2 _returnvalue_4) -1)
            _)
          (`KismetArrayLibrary.Array_Add` (`self.padChoosed`) _returnvalue_4))))
    (else
      (for _index_2 (range 1 (+ (`KismetMathLibrary.FTrunc` (+ (`KismetMathLibrary.Conv_IntToDouble` 5) (/ (`KismetMathLibrary.Conv_IntToDouble` (`self.timePlayed`)) 20.0))) 1))
        (if (== _index_2 1)
          (`KismetArrayLibrary.Array_Add` _padchoosed _returnvalue_3)
          (else
            (while (== (`KismetArrayLibrary.Array_Find` _padchoosed _returnvalue_3) -1)
              _)
            (`KismetArrayLibrary.Array_Add` (`self.padChoosed`) _returnvalue_3))))
      (for _array_element (`self.padChoosed`)
        (`/Game/Blueprints/Objects/ObjectPad.ActivePad` (`|GetArrayItem` (`self.padListReferences`) (`KismetArrayLibrary.Array_Find` (`self.padListCoords`) _array_element)))))))